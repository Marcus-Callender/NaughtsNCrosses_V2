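; BP_CirclePiece is a clickable board-game cell that, when unclaimed, takes BP_GameBoard's current colour and notifies the board.
; Timelines drive material parameters for hover brightness and red or blue claim animations, which also tint the piece below green.
; Construction finds right and bottom neighbours by world-space X/Z position; BeginPlay back-links left and top, then derives diagonals.
; F_Reset restores the unclaimed look; further neighbour-highlight chains are unconnected.
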(event `self.SM_BaseCircle.OnClicked`
  (params (TouchedComponent :type "PrimitiveComponent Object Reference") (ButtonPressed :type "Key Structure" :default "AnyKey"))
  (bind _sm_basecircle (`/Game/Assets/Blueprints/BP_CirclePiece.SM_BaseCircle` (`self.m_bottomNode`)))
  (if (and (`/Game/Assets/Blueprints/BP_GameBoard.m_canClick` (`self.m_pGameBoard`)) (`|EnumEquality` (`self.m_myColour`) "NewEnumerator0"))
    (`/Game/Assets/Blueprints/BP_GameBoard.PieceClicked` (`self.m_pGameBoard`))
    (set `self.m_myColour` (`/Game/Assets/Blueprints/BP_GameBoard.m_currentColour` (`self.m_pGameBoard`)))
    (if (`|EnumEquality` (`self.m_myColour`) "NewEnumerator1")
      (bind (_direction _colourintensity) (`Timeline|Timeline_0` :!via `PlayFromStart`)
        (:`Update`
          (if (`|EnumInequality` (`self.m_myColour`) "NewEnumerator0")
            (`MeshComponent.SetVectorParameterValueOnMaterials` (`self.SM_BaseCircle`) "Colour" (`KismetMathLibrary.MakeVector` _colourintensity))
            (`/Engine/EditorBlueprintResources/StandardMacros.IsValid` _sm_basecircle :!label _label
              (:`Is Valid`
                (`MeshComponent.SetVectorParameterValueOnMaterials` _sm_basecircle "Colour" (`KismetMathLibrary.MakeVector` 0.0 1.0)))))))
      (elif (`|EnumEquality` (`self.m_myColour`) "NewEnumerator2")
        (bind (_direction_2 _colourintensity_2) (`Timeline|TL_ColourChange` :!via `PlayFromStart`)
          (:`Update`
            (if (`|EnumInequality` (`self.m_myColour`) "NewEnumerator0")
              (`MeshComponent.SetVectorParameterValueOnMaterials` (`self.SM_BaseCircle`) "Colour" (`KismetMathLibrary.MakeVector` 0.0 0.0 _colourintensity_2))
              (goto _label))))))))

(event `self.SM_BaseCircle.OnBeginCursorOver`
  (params (TouchedComponent :type "PrimitiveComponent Object Reference"))
  (if (`|EnumEquality` (`self.m_myColour`) "NewEnumerator0")
    (bind (_direction _brightness) (`Timeline|Timeline_1` :!label _label_2)
      (:`Update`
        (`MeshComponent.SetScalarParameterValueOnMaterials` (`self.SM_BaseCircle`) "colourIntensity" (`KismetMathLibrary.Lerp` 5.0 15.0 _brightness))))))

(event `self.ReceiveBeginPlay`
  (`self.GiveSelfAsNode`
    (:`Out`
      (`self.AssignDiaginalNode`))))

(event `self.SM_BaseCircle.OnEndCursorOver`
  (params (TouchedComponent :type "PrimitiveComponent Object Reference"))
  (if (`|EnumEquality` (`self.m_myColour`) "NewEnumerator0")
    (goto _label_2 :!via `Reverse`)))

(fn `F_GiveLeftNode`
  (params (Node :type "/Game/Assets/Blueprints/BP_CirclePiece Object Reference"))
  (set `self.m_leftNode` Node))

(fn `F_GiveTopNode`
  (params (Node :type "/Game/Assets/Blueprints/BP_CirclePiece Object Reference"))
  (set `self.m_topNode` Node))

(fn `F_Reset`
  (bind _tl_colourchange (`self.TL_ColourChange`))
  (set `self.m_myColour` "NewEnumerator0")
  (`TimelineComponent.SetPlaybackPosition` _tl_colourchange 0.0 false false)
  (`TimelineComponent.Stop` _tl_colourchange)
  (`MeshComponent.SetScalarParameterValueOnMaterials` (`self.SM_BaseCircle`) "colourIntensity" 5.0)
  (`MeshComponent.SetVectorParameterValueOnMaterials` (`self.SM_BaseCircle`) "Colour" (`KismetMathLibrary.MakeVector` 0.1 0.1 0.1)))

(fn `UserConstructionScript`
  (locals (m_myID :type Integer :default 100))
  (bind _outactors (`GameplayStatics.GetAllActorsOfClass` "/Game/Assets/Blueprints/BP_GameBoard.BP_GameBoard_C"))
  (set `self.m_pGameBoard` (`KismetArrayLibrary.Array_Get` _outactors))
  (`self.AssignAdjasentNodes`))