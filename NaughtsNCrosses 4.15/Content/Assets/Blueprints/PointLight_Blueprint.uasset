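; PointLight_Blueprint is a point light that tints red or blue to match the current colour state of the game board.
; The construction script caches the first BP_GameBoard found in the level.
; Every Tick checks the board's MCurrentColour and restarts either the red or blue timeline.
; Each timeline's Update sets a fixed light colour without using any track value, so no blend is computed.
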(event `self.ReceiveTick`
  (params (DeltaSeconds :type "Float (single-precision)"))
  (if (`|EnumEquality` (`/Game/Assets/Blueprints/BP_GameBoard.m_currentColour` (`self.m_pGameBoard`)) "NewEnumerator1")
    (`Timeline|TL_ColourChangeRed` :!via `PlayFromStart`
      (:`Update`
        (`LightComponent.SetLightColor` (`self.PointLightComponent`) (make `LinearColor` 1.0 0.5 0.5) true)))
    (else
      (`Timeline|TL_ColourChangeBlue` :!via `PlayFromStart`
        (:`Update`
          (`LightComponent.SetLightColor` (`self.PointLightComponent`) (make `LinearColor` 0.5 0.5 1.0) true))))))

(fn `UserConstructionScript`
  (bind _outactors (`GameplayStatics.GetAllActorsOfClass` "/Game/Assets/Blueprints/BP_GameBoard.BP_GameBoard_C"))
  (set `self.m_pGameBoard` (`KismetArrayLibrary.Array_Get` _outactors)))