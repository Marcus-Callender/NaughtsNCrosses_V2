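; Game board for a two-colour, turn-based line game that spawns a grid of BP_CirclePiece actors on BeginPlay.
; PieceClicked locks clicking, runs CheckVictory, then either announces the winner and resets or swaps the current colour.
; Victory checks walk each piece's neighbour references for five matching colours horizontally, vertically or diagonally.
; Neighbour linking is stubbed or uncalled here, and the draw check is disconnected.
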(event `PieceClicked`
  (set `self.m_canClick` false)
  (`KismetSystemLibrary.Delay` 0.5)
  (`self.CheckVictory`
    (:`Out`
      (if (`self.m_gameWon`)
        (`KismetSystemLibrary.Delay` 1.0)
        (`KismetSystemLibrary.PrintText` (`KismetTextLibrary.Conv_StringToText` (`|GetEnumeratorNameAsString` (`self.m_currentColour`))) true true (struct :`R` 1.0 :`G` 1.0 :`B` 1.0 :`A` 1.0) 5.0)
        (`self.ResetGame`)
        (else
          (if (`|EnumEquality` (`self.m_currentColour`) "NewEnumerator1")
            (set `self.m_currentColour` "NewEnumerator2")
            (else
              (set `self.m_currentColour` "NewEnumerator1")))
          (set `self.m_canClick` true))))))

(event `self.ReceiveBeginPlay`
  (for _index (range (+ (`self.m_horisontalNodes`) 1))
    (for _index_2 (range (+ (`self.m_verticalNodes`) 1))
      (bind _returnvalue (`|SpawnActorFromClass` "/Game/Assets/Blueprints/BP_CirclePiece.BP_CirclePiece_C" (`KismetMathLibrary.Conv_VectorToTransform` (+ (`self.m_startingPosition`) (`KismetMathLibrary.MakeVector` (* _index (`self.m_horizontalNodeOffset`)) 0.0 (* _index_2 (`self.m_verticalNodeOffset`))))) "Undefined" "OverrideRootScale"))
      (`KismetArrayLibrary.Array_Add` (`self.m_nodeList`) _returnvalue)
      (if (!= _index (`self.m_horisontalNodes`))
        _)))
  (for _index_3 (range (+ (`self.m_horisontalNodes`) 1))
    (for _index_4 (range (+ (`self.m_verticalNodes`) 1))
      (if true
        _))))

(fn `FindConnectedNodes`
  (params (Node :type "/Game/Assets/Blueprints/BP_CirclePiece Object Reference") (VerticalPlace :type Integer) (HorizontalPlace :type Integer) (NodeList :type "Array of /Game/Assets/Blueprints/BP_CirclePiece Object Reference")))

(fn `UserConstructionScript`)